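; Door Blueprint that toggles between open and closed states.
; ToggleOpen flips the IsOpen flag and calls OpenDoor or CloseDoor to match.
; Both events only set the visibility of DoorBody, hiding it when open and showing it when closed, with no animation or collision change.
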(event `ToggleOpen`
  (if (`self.IsOpen`)
    (set `self.IsOpen` false)
    (`self.Close Door`)
    (else
      (set `self.IsOpen` true)
      (`self.Open Door`))))

(event `Open Door`
  (`SceneComponent.SetVisibility` (`self.DoorBody`) false false))

(event `Close Door`
  (`SceneComponent.SetVisibility` (`self.DoorBody`) true false))

(fn `UserConstructionScript`)